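; Ranged RetroFPS enemy with Paper2D flipbook visuals, driven by a behavior tree started on its AI controller.
; While it can see the player, Tick turns it to face them on yaw only.
; RangedAttack spawns a projectile, calls a flat ApplyDamage immediately rather than on impact, and briefly blocks further attacks.
; Any damage is fatal, playing death and corpse flipbooks before destroying the actor; MeleeAttack is an empty stub.
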(event Custom|Melee%20Attack)

(event Custom|Ranged%20Attack
  (Game|SpawnActorfromClass "/Game/RetroFPS/Enemy/Projectiles/BP_FirstPersonProjectile.BP_FirstPersonProjectile_C" (Transformation|GetWorldTransform (Variables|Default|GetSpawnProjectileLocation)) "Undefined" "MultiplyWithRoot" 0 0)
  (Utilities|Casting|CastToBP_FPSPlayer (Game|Player|GetPlayerPawn 0))
  (Game|Damage|ApplyDamage 0 3.0 0 0)
  (Variables|Default|Setcanattack false)
  (Utilities|FlowControl|Delay 0.5)
  (Variables|Default|Setcanattack true))

(event EventBeginPlay
  (bind _asbp_retro_fpsenemy_ai (Utilities|Casting|CastToBP_RetroFPSEnemyAI (Pawn|GetController)))
  (AI|RunBehaviorTree _asbp_retro_fpsenemy_ai (Variables|Default|GetBehaviour%20Tree)))

(event EventTick
  (params (DeltaSeconds :type Float%20%28single-precision%29))
  ;[0 0 0] Sprite Rotation
  (if (Variables|Default|Getcanseeplayer)
    (Transformation|SetActorRotation (Math|Rotator|MakeRotator 0.0 0.0 (.yaw (Math|Rotator|FindLookatRotation (Transformation|GetActorLocation) (Transformation|GetActorLocation (Game|GetPlayerCharacter 0))))))))

(event Game|Damage|EventAnyDamage
  (params (Damage :type Float%20%28single-precision%29) (DamageType :type Damage%20Type%20Object%20Reference) (InstigatedBy :type Controller%20Object%20Reference) (DamageCauser :type Actor%20Object%20Reference))
  (bind _paperflipbook (Variables|Default|GetPaperFlipbook))
  ;[0 0 0] Death Sprite
  (Utilities|FlowControl|DoOnce false
    (:Completed
      (Components|Activation|Deactivate (Variables|Character|GetCharacterMovement))
      (Sprite|SetFlipbook _paperflipbook "/Game/RetroFPS/Enemy/Meleedeath1.Meleedeath1")
      (Utilities|FlowControl|Delay (Class|PaperFlipbookComponent|GetFlipbookLength _paperflipbook))
      (Sprite|SetFlipbook (Variables|Default|GetPaperFlipbook) "/Game/RetroFPS/Enemy/Deadbody.Deadbody")
      (Utilities|FlowControl|Delay 1.0)
      (Actor|DestroyActor))))

(fn ConstructionScript)
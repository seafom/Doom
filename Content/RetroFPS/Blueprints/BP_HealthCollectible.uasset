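; BP_HealthCollectible is a health pickup that adds a small amount of health to the FPS player on overlap.
; Tick billboards the pickup toward the player camera using yaw only.
; BeginPlay caches the player, and the trigger's DoOnce-gated overlap clamps the new health, refreshes the HUD with a hard-coded maximum, then destroys the actor.
; An unconnected tag-based IncreaseHealth path remains but never runs.
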(event OnComponentBeginOverlap(Trigger)
  (params (OverlappedComponent :type Primitive%20Component%20Object%20Reference) (OtherActor :type Actor%20Object%20Reference) (OtherComp :type Primitive%20Component%20Object%20Reference) (OtherBodyIndex :type Integer) (bFromSweep :type Boolean) (SweepResult :type Hit%20Result%20Structure%20%28by%20ref%29))
  (bind _as_bp_fpsplayer (Variables|Default|GetAs%20BP%20FPSPlayer))
  (if (== OtherActor (Variables|Default|GetAs%20BP%20FPSPlayer))
    (Utilities|FlowControl|DoOnce (< (Variables|/Game/RetroFPS/Blueprints/BP_FPSPlayer.BP_FPSPlayer_C|GetCurrentHealth (Variables|Default|GetAs%20BP%20FPSPlayer)) 1.0)
      (:Completed
        (if true
          (bind _output_get (Variables|/Game/RetroFPS/Blueprints/BP_FPSPlayer.BP_FPSPlayer_C|SetCurrentHealth _as_bp_fpsplayer (Math|Float|Clamp(Float) (+ (Variables|/Game/RetroFPS/Blueprints/BP_FPSPlayer.BP_FPSPlayer_C|GetCurrentHealth _as_bp_fpsplayer) 1.0) 0.0 (Variables|/Game/RetroFPS/Blueprints/BP_FPSPlayer.BP_FPSPlayer_C|GetMaxHealth _as_bp_fpsplayer))))
          (Default|UpdateHealthUI (Variables|/Game/RetroFPS/Blueprints/BP_FPSPlayer.BP_FPSPlayer_C|GetWB_HUD (Variables|Default|GetAs%20BP%20FPSPlayer)) _output_get 1e+02)
          (Actor|DestroyActor))))))

(event EventTick
  (params (DeltaSeconds :type Float%20%28single-precision%29))
  (bind _healthcollectible (Variables|Default|GetHealthCollectible))
  (Transformation|SetWorldRotation _healthcollectible (Math|Rotator|MakeRotator 0.0 0.0 (- (.yaw (Math|Rotator|FindLookatRotation (Transformation|GetWorldLocation _healthcollectible) (Camera|GetCameraLocation (Game|GetPlayerCameraManager 0)))) 9e+01)) false false))

(event EventBeginPlay
  (bind _asbp_fpsplayer (Utilities|Casting|CastToBP_FPSPlayer (Game|GetPlayerCharacter 0)))
  (Variables|Default|SetAs%20BP%20FPSPlayer _asbp_fpsplayer))

(fn ConstructionScript)
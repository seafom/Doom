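; First-person player character for a retro FPS, handling movement, mouse look, shooting and health.
; EquipWeapon swaps the weapon Child Actor's class, initializes it through the IPlayerWeapon interface and plays its draw sequence.
; Tick drives weapon bobbing from movement velocity, and the shoot input forwards to the current weapon.
; Damage updates the HUD, spawns an explosion effect and triggers Death at zero health, which currently only sets a flag.
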(event Custom|Equip%20Weapon
  (params (Weapon :type BP%20Player%20Weapon%20Base%20Class%20Reference))
  (bind _childactor (Variables|/Script/Engine.ChildActorComponent|GetChildActor (Variables|Default|GetWeapon)))
  ;[0 0 0] Equip Weapon
  (bind _output_get (Variables|Player|SetCurrent%20Weapon Weapon))
  (ChildActorComponent|SetChildActorClass (Variables|Default|GetWeapon) _output_get)
  (if (Utilities|DoesObjectImplementInterface _childactor "/Game/RetroFPS/Blueprints/IPlayerWeapon.IPlayerWeapon_C")
    (Class|IPlayerWeapon|InitializeWeapon(Message) _childactor)
    (bind _asbp_player_weapon_base (Utilities|Casting|CastToBP_PlayerWeaponBase _childactor))
    (bind _output_get_2 (Variables|Default|SetCurrentWeapon _asbp_player_weapon_base))
    (Sequencer|Player|Play (Variables|/Script/ActorSequence.ActorSequenceComponent|GetSequencePlayer (Variables|/Game/RetroFPS/Blueprints/BP_PlayerWeaponBase.BP_PlayerWeaponBase_C|GetWeapon%20Draw _output_get_2)) :!class /Script/MovieScene.MovieSceneSequencePlayer)))

(event Custom|Death
  ;[0.9566 0 0.2012] Death (Add load to Game Over Menu)
  (Variables|Default|SetbDeath true))

(event EventBeginPlay
  (bind _returnvalue (UserInterface|CreateWidget "/Game/RetroFPS/Blueprints/WBP_HUD.WBP_HUD_C"))
  (bind _output_get (Variables|Default|SetWB_HUD _returnvalue))
  (UserInterface|Viewport|AddtoViewport _output_get 0)
  (CallFunction|EquipWeapon "/Game/RetroFPS/Blueprints/BP_PlayerWeaponBase.BP_PlayerWeaponBase_C")
  (UserInterface|CreateWidget "/Game/RetroFPS/Blueprints/WBP_HUD.WBP_HUD_C" (Game|GetPlayerController 0))
  (bind _output_get_2 (Variables|Default|SetCurrentHealth (Variables|Default|GetMaxHealth)))
  (Default|UpdateHealthUI (Variables|Default|GetWB_HUD) _output_get_2 (Variables|Default|GetMaxHealth)))

(event EventTick
  (params (DeltaSeconds :type Float%20%28single-precision%29))
  (bind _asbp_player_weapon_base (Utilities|Casting|CastToBP_PlayerWeaponBase (Variables|/Script/Engine.ChildActorComponent|GetChildActor (Variables|Default|GetWeapon))))
  (Default|WeaponBobbing _asbp_player_weapon_base (> (Math|Vector|VectorLength (Variables|/Script/Engine.MovementComponent|GetVelocity (Variables|Character|GetCharacterMovement))) 0.0) DeltaSeconds))

(event Game|Damage|EventAnyDamage
  (params (Damage :type Float%20%28single-precision%29) (DamageType :type Damage%20Type%20Object%20Reference) (InstigatedBy :type Controller%20Object%20Reference) (DamageCauser :type Actor%20Object%20Reference))
  ;[0 0 0] Health
  (if (not (Variables|Default|GetbDeath))
    (bind _output_get (Variables|Default|SetCurrentHealth (Math|Float|Clamp(Float) (- (Variables|Default|GetCurrentHealth) Damage) 0.0 (Variables|Default|GetMaxHealth))))
    (Default|UpdateHealthUI (Variables|Default|GetWB_HUD) _output_get (Variables|Default|GetMaxHealth))
    (Effects|SpawnEmitteratLocation "/Game/StarterContent/Particles/P_Explosion.P_Explosion" (Transformation|GetActorLocation)) ; When taking damage an fx play (maybe change it)
    (if (== (Variables|Default|GetCurrentHealth) 0.0)
      (CallFunction|Death))))

(event Input|ActionEvents|InputActionShooting
  (params (Key :type Key%20Structure :default "None"))
  ;[0 0 0] Shoot
  (:Pressed
    (Default|ShootWeapon (Variables|Default|GetCurrentWeapon))))

(event Input|AxisEvents|InputAxisHorizontalMovement
  (params (AxisValue :type Float%20%28single-precision%29))
  ;[0 0 0] Movement
  (Pawn|Input|AddMovementInput (Math|Vector|GetRightVector (Math|Rotator|MakeRotator 0.0 0.0 (.yaw (Pawn|GetControlRotation :!class /Script/Engine.Pawn)))) AxisValue false))

(event Input|AxisEvents|InputAxisVerticalMovement
  (params (AxisValue :type Float%20%28single-precision%29))
  ;[0 0 0] Movement
  (Pawn|Input|AddMovementInput (Math|Vector|GetForwardVector (Math|Rotator|MakeRotator 0.0 0.0 (.yaw (Pawn|GetControlRotation :!class /Script/Engine.Pawn)))) AxisValue false))

(event Input|AxisEvents|InputAxisMouseLookVertical
  (params (AxisValue :type Float%20%28single-precision%29))
  ;[0 0 0] Mouse Look
  (Pawn|Input|AddControllerPitchInput AxisValue))

(event Input|AxisEvents|InputAxisMouseLookHorizontal
  (params (AxisValue :type Float%20%28single-precision%29))
  ;[0 0 0] Mouse Look
  (Pawn|Input|AddControllerYawInput AxisValue))

(fn ConstructionScript)
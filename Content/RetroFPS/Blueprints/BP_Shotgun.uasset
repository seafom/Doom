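; Shotgun weapon for a retro FPS that animates firing and reloading with Paper2D flipbooks.
; Initialization shows the idle flipbook and unhides the weapon sprite.
; Shooting calls FireWeapon, then plays fire and reload flipbooks with their sounds, sequenced by delays timed to a fixed interval and the reload flipbook's length.
; It then restores the idle flipbook and calls Resetweapon, which is empty here.
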(event Custom|Resetweapon)

(event EventShootWeapon
  (bind _weapon_flipbook (Variables|Default|GetWeapon%20Flipbook))
  (CallFunction|FireWeapon)
  (Sprite|SetFlipbook _weapon_flipbook "/Game/RetroFPS/Flipbooks/FP_Shotgun_Fire.FP_Shotgun_Fire")
  (Audio|PlaySoundatLocation "/Game/RetroFPS/Sounds/shotgun_fire.shotgun_fire" (Transformation|GetActorLocation) "0, 0, 0" 1.0 1.0 0.0 0 0 0 0)
  (Utilities|FlowControl|Delay 0.2)
  (Sprite|SetFlipbook (Variables|Default|GetWeapon%20Flipbook) "/Game/RetroFPS/Textures/Weapons/PF_Reload.PF_Reload")
  (Audio|PlaySoundatLocation "/Game/RetroFPS/Sounds/shotgun_reload.shotgun_reload" (Transformation|GetActorLocation) "0, 0, 0" 1.0 1.0 0.0 0 0 0 0)
  (Utilities|FlowControl|Delay (Class|PaperFlipbookComponent|GetFlipbookLength _weapon_flipbook))
  (Sprite|SetFlipbook (Variables|Default|GetWeapon%20Flipbook) "/Game/RetroFPS/Flipbooks/FB_Shotgun_Idle.FB_Shotgun_Idle")
  (CallFunction|Resetweapon))

(event EventInitializeWeapon
  (Sprite|SetFlipbook (Variables|Default|GetWeapon%20Flipbook) (Variables|Default|GetIdle%20Shotgun))
  (Development|SetHiddeninGame (Variables|Default|GetWeapon%20Flipbook) false false))

(fn ConstructionScript
  (|CallParentFunction))